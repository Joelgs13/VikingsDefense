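; Tower defense game mode that tracks money and lives and handles defeat, restart and quit.
; BeginPlay shows the mouse cursor and interface widget, while events adjust Money; PlaceTurret is an empty stub.
; DecrementLives sets Lives to zero minus damage instead of subtracting from Lives, so any non-negative damage calls Defeat.
; Defeat freezes time dilation and shows the defeat widget; Restartgame restores time and reopens NewMap.
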(event Custom|DecrementLives
  (params (EnemyDamage :type Integer))
  (bind _output_get (Variables|Default|SetLives (- 0 EnemyDamage)))
  (if (<= _output_get 0)
    (CallFunction|Defeat)))

(event Custom|Defeat
  (Development|PrintString "DEFEAT")
  (Viewport|RemoveAllWidgets)
  (Utilities|Time|SetGlobalTimeDilation 0.0)
  (bind _returnvalue (UserInterface|CreateWidget "/Game/TowerDefense/BluePrints/Interfaces/WBP_Defeat.WBP_Defeat_C"))
  (UserInterface|Viewport|AddtoViewport _returnvalue 0))

(event Custom|IncrementMoney
  (params (RecivedMoney :type Integer))
  (Variables|Default|SetMoney (+ (Variables|Default|GetMoney) RecivedMoney)))

(event Custom|Restartgame
  (Utilities|Time|SetGlobalTimeDilation 1.0)
  (Game|OpenLevel(byObjectReference) "/Game/TowerDefense/NewMap.NewMap"))

(event Custom|DecrementMoney
  (params (Cost :type Integer))
  (Variables|Default|SetMoney (- (Variables|Default|GetMoney) Cost)))

(event Custom|PlaceTurret)

(event Custom|Exit%20Game
  (Game|QuitGame 0 "Quit" false))

(event EventBeginPlay
  (bind _returnvalue (Game|GetPlayerController 0))
  (Variables|/Script/Engine.PlayerController|SetbShowMouseCursor _returnvalue true)
  (Input|SetInputModeGameandUI _returnvalue 0 "DoNotLock" false false)
  (bind _returnvalue_2 (UserInterface|CreateWidget "/Game/TowerDefense/BluePrints/Interfaces/WBP_Interface.WBP_Interface_C"))
  (UserInterface|Viewport|AddtoViewport _returnvalue_2 0))

(fn ConstructionScript)