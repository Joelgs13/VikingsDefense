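; BP_BaseEnemy is the tower defense base enemy, which moves to a destination and can be destroyed by damage.
; On possession it caches its AIC_Enemy controller, waits a tick, then tells it to move to Destination.
; Health starts at MaxHP in the construction script.
; AnyDamage sets CurrentHP to Damage minus CurrentHP (operands reversed from a usual subtraction) and destroys the actor at zero or below.
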(event EventBeginPlay)

(event Collision|EventActorBeginOverlap
  (params (OtherActor :type Actor%20Object%20Reference)))

(event EventTick
  (params (DeltaSeconds :type Float%20%28single-precision%29)))

(event EventPossessed
  (params (NewController :type Controller%20Object%20Reference))
  (bind _asaic_enemy (Utilities|Casting|CastToAIC_Enemy NewController))
  (Variables|Default|SetAs%20AIC%20Enemy _asaic_enemy)
  (Utilities|FlowControl|DelayUntilNextTick)
  (Default|MovetoGoalLocation (Variables|Default|GetAs%20AIC%20Enemy) (Variables|Default|GetDestination)))

(event Game|Damage|EventAnyDamage
  (params (Damage :type Float%20%28single-precision%29) (DamageType :type Damage%20Type%20Object%20Reference) (InstigatedBy :type Controller%20Object%20Reference) (DamageCauser :type Actor%20Object%20Reference))
  (bind _output_get (Variables|Default|SetCurrentHP (- Damage (Variables|Default|GetCurrentHP))))
  (if (<= _output_get 0.0)
    (Actor|DestroyActor)))

(fn ConstructionScript
  (Variables|Default|SetCurrentHP (Variables|Default|GetMaxHP)))