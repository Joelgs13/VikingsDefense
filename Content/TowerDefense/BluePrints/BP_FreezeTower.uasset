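; BP_FreezeTower is a tower defense tower that shoots homing projectiles and freezes enemies in its range.
; Its Shoot event spawns a BP_FreezeProjectile at the Sphere's transform, passing Damage and homing it on the first enemy in EnemiesRange.
; It calls FreezeTime on that enemy at launch, not on impact.
; It then moves that enemy to the array's end, rotating targets to avoid repeatedly hitting the same one.
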(event EventShoot
  (bind _enemiesrange (Variables|Default|GetEnemiesRange))
  (bind _output (Utilities|Array|Get(acopy) _enemiesrange))
  ;[0.15 0.15 0.15 0.5] Spawn de los proyectiles
  (bind _returnvalue (Game|SpawnActorfromClass "/Game/TowerDefense/BluePrints/BP_FreezeProjectile.BP_FreezeProjectile_C" (Transformation|GetWorldTransform (Variables|Default|GetSphere)) "AlwaysSpawn" "OverrideRootScale" self (Variables|Default|GetDamage) self))
  (Variables|/Script/Engine.ProjectileMovementComponent|SetHomingTargetComponent (Variables|/Game/TowerDefense/BluePrints/BP_BaseProjectile.BP_BaseProjectile_C|GetProjectileMovement _returnvalue) (Variables|/Script/Engine.Character|GetCapsuleComponent (Utilities|Array|Get(acopy) (Variables|Default|GetEnemiesRange))))
  ;[0.15 0.15 0.15 0.5] se aplica el evento de congelar
  (Default|FreezeTime _output (Variables|Default|GetFreezeDuration))
  ;[0.15 0.15 0.15 0.5] se añade al array si se descongela
  (Utilities|Array|Add _enemiesrange _output)
  ;[0.15 0.15 0.15 0.5] Se quita del array evita disparar al mismo continuamente
  (Utilities|Array|RemoveIndex _enemiesrange))

(fn ConstructionScript
  (|CallParentFunction))