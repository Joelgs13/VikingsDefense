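; Tower defense tower meant to deal gradually increasing damage to the first enemy in its range list.
; Each Shoot raises Damage up to a cap, applies it directly without projectiles, then calls EnemyIsDead on the target with its current HP.
; Damage currently resets after any shot with a valid target, defeating the ramp; a note marks this to change to reset only on target switch.
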(event EventBeginPlay)

(event EventShoot
  (bind _output_get (Variables|Default|SetActualEnemy (Utilities|Array|Get(acopy) (Variables|Default|GetEnemiesRange))))
  (if (>= (Variables|Default|GetDamage) 5e+01)
    (Variables|Default|SetDamage 5e+01)
    (else
      (bind _output_get_2 (Variables|Default|SetDamage (+ (Variables|Default|GetDamage) 3.0)))
      ;[0.15 0.15 0.15 0.5] borrar
      (Development|PrintString (Utilities|String|ToString(Float) _output_get_2))))
  ;[0.15 0.15 0.15 0.5] Spawn de los proyectiles
  (Game|Damage|ApplyDamage _output_get (Variables|Default|GetDamage) (Game|GetInstigatorController) self "/Script/Engine.DamageType")
  (bind _actualenemy (Variables|Default|GetActualEnemy)
    (:then
      (Default|EnemyIsDead _actualenemy (Variables|/Game/TowerDefense/BluePrints/BP_BaseEnemy.BP_BaseEnemy_C|GetCurrentHP _actualenemy))
      ;[0.15 0.15 0.15 0.5] cambiar esto para que solo reinicie el daño al cambiar de objetivo
      (Variables|Default|SetDamage 1.0))
    (:else)))

(fn ConstructionScript)

(fn DealDamagetoEnemies)