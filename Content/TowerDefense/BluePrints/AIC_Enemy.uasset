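; AI controller for tower defense enemies that walks its possessed BP_BaseEnemy to a goal location.
; It caches the GM_TowerDefense game mode on begin play and the enemy pawn on possess, then runs AI Move To when MoveToGoalLocation is called.
; Reaching the goal subtracts the enemy's damage from lives, decrements the enemy count and destroys the enemy; failure prints a debug message.
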(event Custom|MoveToGoalLocation
  (params (Destination :type Vector))
  (bind _movementresult (AI|AIMoveTo (Variables|Default|GetBP_BaseEnemy) Destination 0 5.0 false)
    (:OnSuccess
      (Default|DecrementLives (Variables|Default|GetGamemode) (Variables|/Game/TowerDefense/BluePrints/Enemies/BP_BaseEnemy.BP_BaseEnemy_C|GetDamage (Variables|Default|GetBP_BaseEnemy)))
      (Default|SubstractEnemy (Variables|Default|GetGamemode))
      (Actor|DestroyActor (Variables|Default|GetBP_BaseEnemy)))
    (:OnFail
      (Development|PrintString (Utilities|String|Append "Movement Failed on " (Utilities|GetDisplayName (Variables|Default|GetBP_BaseEnemy)) "Cause " (Utilities|String|EnumtoString _movementresult)) true true "(R=1.000000,G=0.144324,B=0.280905,A=1.000000)" 1e+01))))

(event EventBeginPlay
  (bind _asgm_tower_defense (Utilities|Casting|CastToGM_TowerDefense (Game|GetGameMode)))
  (Variables|Default|SetGamemode _asgm_tower_defense))

(event EventPossess
  (params (PossessedPawn :type Pawn%20Object%20Reference))
  (bind _asbp_base_enemy (Utilities|Casting|CastToBP_BaseEnemy PossessedPawn))
  (Variables|Default|SetBP_BaseEnemy _asbp_base_enemy))

(fn ConstructionScript)