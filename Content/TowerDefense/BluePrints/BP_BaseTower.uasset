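; Base tower actor for a tower defense game that automatically fires homing projectiles at enemies within range.
; Sphere overlaps add and remove BP_BaseEnemy actors in the EnemiesRange list.
; The first enemy starts a looping Shoot timer, which pauses when the list empties and resumes on a new entry.
; Each shot spawns a BP_BaseProjectile with the tower's Damage, homing on the first listed enemy's capsule.
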(event OnComponentBeginOverlap(Sphere)
  (params (OverlappedComponent :type Primitive%20Component%20Object%20Reference) (OtherActor :type Actor%20Object%20Reference) (OtherComp :type Primitive%20Component%20Object%20Reference) (OtherBodyIndex :type Integer) (bFromSweep :type Boolean) (SweepResult :type Hit%20Result%20Structure%20%28by%20ref%29))
  ;[0.15 0.15 0.15 0.5] Funcion de disparar solo a los enemigos mientras esta dentro del radio de accion
  ;;[0.15 0.15 0.15 0.5] Se lanza el evento cuando ocurre el overlap
  ;;[0.15 0.15 0.15 0.5] comprueba que sea un enemigo
  (bind _asbp_base_enemy (Utilities|Casting|CastToBP_BaseEnemy OtherActor))
  (Utilities|Array|AddUnique (Variables|Default|GetEnemiesRange) _asbp_base_enemy)
  (if (Utilities|Time|IsValidTimerHandle (Variables|Default|GetShooterTimerhandle))
    (if (Utilities|Time|IsTimerActivebyHandle (Variables|Default|GetShooterTimerhandle))
      (Variables|Default|SetIsShooting (not (Variables|Default|GetIsShooting)))
      (else
        (Utilities|Time|UnpauseTimerbyHandle (Variables|Default|GetShooterTimerhandle))))
    (else
      ;;[0.15 0.15 0.15 0.5] Se establece un temporizador
      (bind _returnvalue (Utilities|Time|SetTimerbyEvent (delegate Custom|Shoot) 0.5 true true))
      ;;[0.15 0.15 0.15 0.5] Se guarda el valor del temporizador en una variable
      (Variables|Default|SetShooterTimerhandle _returnvalue))))

(event OnComponentEndOverlap(Sphere)
  (params (OverlappedComponent :type Primitive%20Component%20Object%20Reference) (OtherActor :type Actor%20Object%20Reference) (OtherComp :type Primitive%20Component%20Object%20Reference) (OtherBodyIndex :type Integer))
  (bind _enemiesrange (Variables|Default|GetEnemiesRange))
  ;[0.15 0.15 0.15 0.5] Funcion de disparar solo a los enemigos mientras esta dentro del radio de accion
  ;;[0.15 0.15 0.15 0.5] Cancela el disparo cuando el overlap del enemigo casteado sale
  ;;;[0.15 0.15 0.15 0.5] Evento cuando se termina el overlap
  ;;;[0.15 0.15 0.15 0.5] se comprueba que sea un enemigo
  (bind _asbp_base_enemy (Utilities|Casting|CastToBP_BaseEnemy OtherActor))
  (Utilities|Array|RemoveItem _enemiesrange _asbp_base_enemy)
  (if (Utilities|Array|IsEmpty _enemiesrange)
    (Utilities|Time|PauseTimerbyHandle (Variables|Default|GetShooterTimerhandle))))

(event Custom|Shoot
  ;[0.15 0.15 0.15 0.5] Funcion de disparar solo a los enemigos mientras esta dentro del radio de accion
  ;;[0.15 0.15 0.15 0.5] Evento de disparar
  ;;[0.15 0.15 0.15 0.5] Spawn de los proyectiles
  (bind _returnvalue (Game|SpawnActorfromClass "/Game/TowerDefense/BluePrints/BP_BaseProjectile.BP_BaseProjectile_C" (Transformation|GetWorldTransform (Variables|Default|GetSphere)) "AlwaysSpawn" "OverrideRootScale" self (Variables|Default|GetDamage) self))
  (Variables|/Script/Engine.ProjectileMovementComponent|SetHomingTargetComponent (Variables|/Game/TowerDefense/BluePrints/BP_BaseProjectile.BP_BaseProjectile_C|GetProjectileMovement _returnvalue) (Variables|/Script/Engine.Character|GetCapsuleComponent (Utilities|Array|Get(acopy) (Variables|Default|GetEnemiesRange)))))

(event EventBeginPlay)

(fn ConstructionScript
  (Variables|Default|SetRange (Variables|Default|GetRange)))