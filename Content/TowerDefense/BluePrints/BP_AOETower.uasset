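; Area-of-effect tower Blueprint for a tower defense game that damages every enemy in its range when it shoots.
; The Shoot event calls DealDamageToEnemies, which copies EnemiesRange into EnemiesArray and applies the tower's Damage to each entry.
; EnemiesArray is never cleared in this graph, so entries from earlier shots can accumulate and be damaged again.
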(event EventBeginPlay)

(event EventShoot
  (CallFunction|DealDamagetoEnemies))

(fn ConstructionScript)

(fn DealDamagetoEnemies
  (bind _enemiesarray (LocalVariables|GetEnemiesArray))
  ;[0.15 0.15 0.15 0.5] cojo todos los ewlentos de mi array, y los meto a otro array de objetos puros
  (for _array_element (Variables|Default|GetEnemiesRange)
    (Utilities|Array|Add _enemiesarray (Utilities|ResolveSoftReference _array_element)))
  ;[0.15 0.15 0.15 0.5] Por cada elemento en el array, le hacemos daño
  (for _array_element_2 _enemiesarray
    (Game|Damage|ApplyDamage (Utilities|ResolveSoftReference _array_element_2) (Variables|Default|GetDamage) (Game|GetInstigatorController) self "/Script/Engine.DamageType")))