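; BP_FireProjectile is a tower defense projectile that deals damage and applies a timed fire effect to enemies on overlap.
; With a valid HomingTarget, the StaticMesh overlap proceeds only if the overlapped component, rather than the other actor, equals that target.
; Without one, any BP_BaseEnemy qualifies.
; A hit applies damage through ApplyDamage, then passes FireTime to the enemy's FireTime call.
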(event OnComponentBeginOverlap(StaticMesh)
  (params (OverlappedComponent :type Primitive%20Component%20Object%20Reference) (OtherActor :type Actor%20Object%20Reference) (OtherComp :type Primitive%20Component%20Object%20Reference) (OtherBodyIndex :type Integer) (bFromSweep :type Boolean) (SweepResult :type Hit%20Result%20Structure%20%28by%20ref%29))
  (bind _homingtarget (Variables|Default|GetHomingTarget)
    (:then
      (if (== OverlappedComponent _homingtarget)
        (Game|Damage|ApplyDamage OtherActor (Variables|Default|GetDamage) (Game|GetInstigatorController) self "/Script/Engine.DamageType" :!label _label)
        (bind _asbp_base_enemy (Utilities|Casting|CastToBP_BaseEnemy OtherActor))
        (if (Utilities|IsValid _asbp_base_enemy)
          (Default|FireTime _asbp_base_enemy (Variables|Default|GetFireTime)))))
    (:else
      (Utilities|Casting|CastToBP_BaseEnemy OtherActor)
      (goto _label))))

(fn ConstructionScript
  (|CallParentFunction))