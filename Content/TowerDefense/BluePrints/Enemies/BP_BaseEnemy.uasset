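; Base enemy for a tower defense game that walks to a goal, takes damage and can be frozen or set burning.
; On possession it has its AIC_Enemy controller move it to the destination next tick.
; Freeze temporarily swaps material and slows movement through a retriggerable delay, while fire adds or restarts a BPC_Burning component.
; Damage reduces HP, and death awards money through the game mode before destroying the actor.
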(event Custom|FreezeTime
  (params (Duration :type Float%20%28single-precision%29))
  ;[0.15 0.15 0.15 0.5] Evento para congelar. Cambia el material y cambia la velocidad maxima
  ;;[0.15 0.15 0.15 0.5] Cambiar material
  (Rendering|Material|SetMaterial (Variables|Character|GetMesh) 1 "/Engine/TemplateResources/MI_Template_BaseGray_02.MI_Template_BaseGray_02")
  ;;[0.15 0.15 0.15 0.5] Cambiar velocidad maxima
  (Variables|/Script/Engine.CharacterMovementComponent|SetMaxWalkSpeed (Variables|Character|GetCharacterMovement) (* (/ (Variables|Default|GetBase%20speed) 1e+02) 15.0))
  ;;[0.15 0.15 0.15 0.5] Delay para evitar que se salte el tiempo de congelacion
  (Utilities|FlowControl|RetriggerableDelay Duration)
  ;;[0.15 0.15 0.15 0.5] Se devuelve el material y la velocidad se reestablece
  (Rendering|Material|SetMaterial (Variables|Character|GetMesh) 1 (Variables|Default|GetBase%20Material))
  (Variables|/Script/Engine.CharacterMovementComponent|SetMaxWalkSpeed (Variables|Character|GetCharacterMovement) (Variables|Default|GetBase%20speed)))

(event Custom|FireTime
  (params (Duration :type Float%20%28single-precision%29))
  (bind _self self)
  (bind _returnvalue (Actor|GetComponentbyClass _self "/Game/TowerDefense/BluePrints/components/BPC_Burning.BPC_Burning_C"))
  ;[0.15 0.15 0.15 0.5] Evento para fuego. Cambia el material y cambia la velocidad maxima y aplica un poco de daño (sin hacer lo del daño)
  (Utilities|IsValid _returnvalue
    (:Is%20Valid
      (Default|(Re)StartDuration _returnvalue))
    (:Is%20Not%20Valid
      (AddComponent|AddBPCBurning _self Duration))))

(event EventPossessed
  (params (NewController :type Controller%20Object%20Reference))
  (bind _asaic_enemy (Utilities|Casting|CastToAIC_Enemy NewController))
  (Variables|Default|SetAs%20AIC%20Enemy _asaic_enemy)
  (Utilities|FlowControl|DelayUntilNextTick)
  (Default|MovetoGoalLocation (Variables|Default|GetAs%20AIC%20Enemy) (Variables|Default|GetDestination)))

(event Game|Damage|EventAnyDamage
  (params (Damage :type Float%20%28single-precision%29) (DamageType :type Damage%20Type%20Object%20Reference) (InstigatedBy :type Controller%20Object%20Reference) (DamageCauser :type Actor%20Object%20Reference))
  (bind _output_get (Variables|Default|SetCurrentHP (- (Variables|Default|GetCurrentHP) Damage)))
  (CallFunction|EnemyIsDead _output_get))

(fn ConstructionScript
  (Variables|Default|SetCurrentHP (Variables|Default|GetMaxHP))
  (Variables|/Script/Engine.CharacterMovementComponent|SetMaxWalkSpeed (Variables|Character|GetCharacterMovement) (Variables|Default|GetBase%20speed)))

(fn EnemyIsDead
  (params (CurrentHP :type Float%20%28double-precision%29))
  (if (<= CurrentHP 0.0)
    ;[0.15 0.15 0.15 0.5] Restar enemigos
    (Default|IncrementMoney (Variables|Default|Getgamemode) (Variables|Default|GetGivedMoney))
    (Variables|Default|SetActual%20Number%20Enemies (- (.ActualNumberEnemies (Utilities|GetClassDefaults "/Game/TowerDefense/BluePrints/BP_EnemySpawner.BP_EnemySpawner_C")) 1))
    (Actor|DestroyActor)))