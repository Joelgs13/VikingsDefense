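; Tower defense enemy spawner that registers with GM_TowerDefense and spawns enemies round by round from SpawnerData.
; Each round runs its groups in sequence, using a looping timer with a start delay to spawn enemies toward Destination.
; It reports each spawn to the game mode and sets SpawnFinish when groups run out; NextRound advances the data index.
; The GetSpawnRate and GetEnemiesInGroup names are swapped: they return enemy count and spawn interval respectively.
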(event Custom|NextRound
  (Variables|/Game/TowerDefense/Gamemode/GM_TowerDefense.GM_TowerDefense_C|SetSpawnFinish (Variables|Default|GetGamemode) false)
  (Math|Integer|IncrementInt (Variables|Default|GetCurrentRound)
    (:%20%20
      (Variables|Default|SetCurrentGroup 0)
      (if (Utilities|Array|IsValidIndex (Variables|config|GetSpawnerData) (Variables|Default|GetCurrentRound))
        (CallFunction|StartGroup)))))

(event Custom|Spawn
  (if (>= (Variables|Default|GetEnemiesSpawnerInCurrentGroup) (CallFunction|GetSpawnRate))
    ;[0.15 0.15 0.15 0.5] En caso de que se complete el spawn de numero pasa al siguente grupo cerrando el timer y añadiendo el valor
    (Utilities|Time|ClearandInvalidateTimerbyHandle (Variables|Default|GetSpawnTimerHandle))
    (Math|Integer|IncrementInt (Variables|Default|GetCurrentGroup)
      (:%20%20
        (Variables|Default|SetEnemiesSpawnerInCurrentGroup 0)
        (CallFunction|StartGroup)))
    (else
      ;[0.15 0.15 0.15 0.5] Spawn del actor y se suma una al numero total del grupo actual
      (bind _returnvalue (Game|SpawnActorfromClass (CallFunction|GetEnemyTypeinGroup) (Transformation|GetActorTransform) "AdjustIfPossibleButAlwaysSpawn" "MultiplyWithRoot" 0 (Transformation|GetWorldLocation (Variables|Default|GetDestination)) 0))
      (Variables|/Game/TowerDefense/BluePrints/Enemies/BP_BaseEnemy.BP_BaseEnemy_C|Setgamemode _returnvalue (Variables|Default|GetGamemode))
      (CallFunction|AddCurrentGroup)
      (Default|NewEnemy (Variables|Default|GetGamemode)))))

(event Custom|StartGroup
  (if (Utilities|Array|IsValidIndex (.groupdata (Utilities|Array|Get(acopy) (Variables|config|GetSpawnerData) (Variables|Default|GetCurrentRound))) (Variables|Default|GetCurrentGroup))
    (bind _returnvalue (Utilities|Time|SetTimerbyEvent (delegate Custom|Spawn) (CallFunction|GetEnemiesinGroup) true false (CallFunction|GetGroupDelay)))
    (Variables|Default|SetSpawnTimerHandle _returnvalue)
    (else
      (Variables|/Game/TowerDefense/Gamemode/GM_TowerDefense.GM_TowerDefense_C|SetSpawnFinish (Variables|Default|GetGamemode) true))))

(event EventBeginPlay
  ;[0.15 0.15 0.15 0.5] Se llama al evento de Start Group
  (bind _asgm_tower_defense (Utilities|Casting|CastToGM_TowerDefense (Game|GetGameMode)))
  (bind _output_get (Variables|Default|SetGamemode _asgm_tower_defense))
  (Variables|/Game/TowerDefense/Gamemode/GM_TowerDefense.GM_TowerDefense_C|SetBP_Spawn _output_get self)
  (EventDispatchers|BindEventtoStartRound (Variables|Default|GetGamemode) (EventDispatchers|CreateEvent :!event Custom|NextRound))
  (CallFunction|StartGroup))

(event Collision|EventActorBeginOverlap
  (params (OtherActor :type Actor%20Object%20Reference)))

(event EventTick
  (params (DeltaSeconds :type Float%20%28single-precision%29)))

(fn ConstructionScript)

(fn GetEnemiesinGroup
  (return (.SpawnRate (Utilities|Struct|BreakS_EnemyGroupData (Utilities|Array|Get(acopy) (.groupdata (Utilities|Array|Get(acopy) (Variables|config|GetSpawnerData) (Variables|Default|GetCurrentRound))) (Variables|Default|GetCurrentGroup))))))

(fn GetEnemyTypeinGroup
  (return (.EnemyType (Utilities|Struct|BreakS_EnemyGroupData (Utilities|Array|Get(acopy) (.groupdata (Utilities|Array|Get(acopy) (Variables|config|GetSpawnerData) (Variables|Default|GetCurrentRound))) (Variables|Default|GetCurrentGroup))))))

(fn GetGroupDelay
  (return (.GroupDelay (Utilities|Struct|BreakS_EnemyGroupData (Utilities|Array|Get(acopy) (.groupdata (Utilities|Array|Get(acopy) (Variables|config|GetSpawnerData) (Variables|Default|GetCurrentRound))) (Variables|Default|GetCurrentGroup))))))

(fn GetSpawnRate
  (return (.EnumEnemies (Utilities|Struct|BreakS_EnemyGroupData (Utilities|Array|Get(acopy) (.groupdata (Utilities|Array|Get(acopy) (Variables|config|GetSpawnerData) (Variables|Default|GetCurrentRound))) (Variables|Default|GetCurrentGroup))))))

(fn AddCurrentGroup
  (Math|Integer|IncrementInt (Variables|Default|GetEnemiesSpawnerInCurrentGroup)))