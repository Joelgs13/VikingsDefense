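; Burning status-effect component for the tower defense game that damages and slows its target unit for a limited time.
; On BeginPlay it swaps a mesh material, cuts walk speed to about two-thirds of base, and starts a looping timer that applies burn damage.
; A retriggerable delay in (Re)StartDuration lets repeat calls refresh the effect; on expiry it restores material and speed, then destroys the component.
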(event Custom|Burn
  (bind _damageunit (Variables|Default|GetDamageUnit))
  (Game|Damage|ApplyDamage _damageunit (Variables|Default|GetBurnDMG) (Game|GetInstigatorController (Variables|Default|GetDamageUnit)) _damageunit)
  (Development|PrintString "IS BURNING")
  (Variables|Default|SetIs%20Burning true))

(event Custom|%28Re%29StartDuration
  (bind _damageunit (Variables|Default|GetDamageUnit))
  (Utilities|FlowControl|RetriggerableDelay (Variables|Default|GetDuration))
  ;[0.15 0.15 0.15 0.5] Se devuelve el material y la velocidad se reestablece
  (Rendering|Material|SetMaterial (Variables|/Script/Engine.Character|GetMesh _damageunit) 1 (Variables|/Game/TowerDefense/BluePrints/BP_BaseEnemy.BP_BaseEnemy_C|GetBase%20Material _damageunit))
  (Variables|/Script/Engine.CharacterMovementComponent|SetMaxWalkSpeed (Variables|/Script/Engine.Character|GetCharacterMovement _damageunit) (Variables|/Game/TowerDefense/BluePrints/BP_BaseEnemy.BP_BaseEnemy_C|GetBase%20speed _damageunit))
  (Components|DestroyComponent))

(event EventBeginPlay
  (bind _damageunit (Variables|Default|GetDamageUnit))
  (Utilities|FlowControl|Sequence
    (:then_0
      ;[0.15 0.15 0.15 0.5] Se devuelve el material y la velocidad se reestablece
      (Rendering|Material|SetMaterial (Variables|/Script/Engine.Character|GetMesh _damageunit) 1 "/Engine/VREditor/LaserPointer/LaserPointerMaterial.LaserPointerMaterial")
      (Variables|/Script/Engine.CharacterMovementComponent|SetMaxWalkSpeed (Variables|/Script/Engine.Character|GetCharacterMovement _damageunit) (* (/ (Variables|/Game/TowerDefense/BluePrints/BP_BaseEnemy.BP_BaseEnemy_C|GetBase%20speed (Variables|Default|GetDamageUnit)) 1e+02) 66.0))
      (if (Utilities|Time|IsValidTimerHandle (Variables|Default|GetBurning%20TimerHandle))
        (if (Utilities|Time|IsTimerActivebyHandle (Variables|Default|GetBurning%20TimerHandle))
          (Variables|Default|SetIs%20Burning (not (Variables|Default|GetIs%20Burning)))
          (else
            (Utilities|Time|UnpauseTimerbyHandle (Variables|Default|GetBurning%20TimerHandle))))
        (else
          ;[0.15 0.15 0.15 0.5] Se establece un temporizador
          (bind _returnvalue (Utilities|Time|SetTimerbyEvent (delegate Custom|Burn) (Variables|Default|GetInterval) true true))
          ;[0.15 0.15 0.15 0.5] Se guarda el valor del temporizador en una variable
          (Variables|Default|SetBurning%20TimerHandle _returnvalue))))
    (:then_1
      (CallFunction|(Re)StartDuration))))