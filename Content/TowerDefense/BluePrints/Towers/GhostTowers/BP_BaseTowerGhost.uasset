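; BP_BaseTowerGhost is the base tower ghost in the tower defense game, showing through its material whether it overlaps an obstacle.
; Mesh overlaps with actors tagged "Obstacle" add them to TowerInRange and switch the mesh to a blocked-state material.
; End overlap removes the actor and restores the green material once the list is empty, so several simultaneous obstacles are handled.
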(event OnComponentBeginOverlap(StaticMesh)
  (params (OverlappedComponent :type Primitive%20Component%20Object%20Reference) (OtherActor :type Actor%20Object%20Reference) (OtherComp :type Primitive%20Component%20Object%20Reference) (OtherBodyIndex :type Integer) (bFromSweep :type Boolean) (SweepResult :type Hit%20Result%20Structure%20%28by%20ref%29))
  (if (Actor|ActorHasTag OtherActor "Obstacle")
    (Utilities|Array|AddUnique (Variables|Default|GetTowerInRange) OtherActor)
    (Rendering|Material|SetMaterial (Variables|Default|GetStaticMesh) 0 "/Engine/VREditor/BasicMeshes/MI_Cube_03.MI_Cube_03")))

(event OnComponentEndOverlap(StaticMesh)
  (params (OverlappedComponent :type Primitive%20Component%20Object%20Reference) (OtherActor :type Actor%20Object%20Reference) (OtherComp :type Primitive%20Component%20Object%20Reference) (OtherBodyIndex :type Integer))
  (bind _towerinrange (Variables|Default|GetTowerInRange))
  (Utilities|Array|RemoveItem _towerinrange OtherActor)
  (if (Utilities|Array|IsEmpty _towerinrange)
    (Rendering|Material|SetMaterial (Variables|Default|GetStaticMesh) 0 "/Engine/EngineDebugMaterials/VertexColorViewMode_GreenOnly.VertexColorViewMode_GreenOnly")))

(event EventBeginPlay)

(fn ConstructionScript)