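; Tower defense tower whose damage ramps up the longer it keeps hitting the same enemy.
; Each Shoot event targets the first enemy in EnemiesRange, resetting damage to a low base when that target differs from the previous one.
; Damage then compounds by a percentage per shot up to a cap and is applied directly with ApplyDamage, without spawning projectiles.
; DealDamageToEnemies is an empty stub.
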(event EventBeginPlay)

(event EventShoot
  (Variables|Default|SetActualEnemy (Utilities|Array|Get(acopy) (Variables|Default|GetEnemiesRange)))
  (if (== (Variables|Default|GetActualEnemy) (Variables|Default|GetPreviousTarget))
    _
    (else
      (Variables|Default|SetDamage 0.2)))
  (if (< (Variables|Default|GetDamage) 5e+01)
    (Variables|Default|SetDamage (+ (Variables|Default|GetDamage) (* (/ (Variables|Default|GetDamage) 1e+02) 12.0)))
    (else
      (Variables|Default|SetDamage 5e+01)))
  ;[0.15 0.15 0.15 0.5] Spawn de los proyectiles
  (Game|Damage|ApplyDamage (Variables|Default|GetActualEnemy) (Variables|Default|GetDamage) (Game|GetInstigatorController) self "/Script/Engine.DamageType")
  (Variables|Default|SetPreviousTarget (Variables|Default|GetActualEnemy)))

(fn ConstructionScript)

(fn DealDamagetoEnemies)