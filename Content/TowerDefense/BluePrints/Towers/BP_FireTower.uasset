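; BP_FireTower is a tower defense tower that fires homing fire projectiles at enemies.
; Its Shoot event spawns a BP_FireProjectile at the Sphere component's transform, passing its Damage and setting itself as owner and instigator.
; The projectile's homing target is set to the capsule of the first entry in EnemiesRange, with no check for an empty list.
; The construction script only calls its parent.
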(event EventShoot
  ;[0.15 0.15 0.15 0.5] Spawn de los proyectiles
  (bind _returnvalue (Game|SpawnActorfromClass "/Game/TowerDefense/BluePrints/Projectiles/BP_FireProjectile.BP_FireProjectile_C" (Transformation|GetWorldTransform (Variables|Default|GetSphere)) "AlwaysSpawn" "OverrideRootScale" self (Variables|Default|GetDamage) self))
  (Variables|/Script/Engine.ProjectileMovementComponent|SetHomingTargetComponent (Variables|/Game/TowerDefense/BluePrints/Projectiles/BP_BaseProjectile.BP_BaseProjectile_C|GetProjectileMovement _returnvalue) (Variables|/Script/Engine.Character|GetCapsuleComponent (Utilities|Array|Get(acopy) (Variables|Default|GetEnemiesRange)))))

(fn ConstructionScript
  (|CallParentFunction))